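; Test game mode that tracks how many objectives remain before a level counts as cleared.
; On BeginPlay it counts every actor implementing BPI_NodeCleared, excluding itself, to set the objective total.
; Each ObjectiveCleared event decrements the count and checks whether it has reached zero or below.
; The count and cleared state are only reported through debug prints.
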(event EventBeginPlay
  (CallFunction|InitObjective))

(event EventObjectiveCleared
  (CallFunction|UpdateNumObjective)
  (Development|PrintString (Utilities|String|ToString(Integer) (Variables|Default|GetnumObjective)))
  (bind _cleared (CallFunction|IsLevelCleared))
  (if _cleared
    (Development|PrintString "Level Cleared")
    (else
      (Development|PrintString "Not cleared yet."))))

(fn ConstructionScript)

(fn InitObjective
  ;[1 1 1] Set the number of objectives in a level.
  (bind _outactors (Actor|GetAllActorswithInterface "/Game/Blueprint/BPI_NodeCleared.BPI_NodeCleared_C"))
  (for _array_element _outactors
    (if (not (== _array_element self)) ; If the sctor is the level BP itself, don't increment.
      (bind _output_get (Variables|Default|SetnumObjective (Variables|Default|GetnumObjective)))
      (Math|Integer|IncrementInt _output_get)))
  ;[1 1 1] Debug
  (Development|PrintString (Utilities|String|ToString(Integer) (Variables|Default|GetnumObjective))))

(fn UpdateNumObjective
  (Math|Integer|DecrementInt (Variables|Default|GetnumObjective)))

(fn IsLevelCleared
  (return (<= (Variables|Default|GetnumObjective) 0)))