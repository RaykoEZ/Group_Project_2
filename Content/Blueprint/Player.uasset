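; Player Blueprint that moves a sprite-based character along the world X and Y axes from input.
; MoveX and MoveY axis events each add the axis value times MoveSpeed to the root component's world location.
; Movement sets the location directly without sweep or delta-time scaling, so it skips blocking collision and varies with frame rate.
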(event Input|AxisEvents|InputAxisMoveX
  (params (AxisValue :type Float%20%28single-precision%29))
  ;[1 1 1] Movement for sprite
  (Transformation|SetWorldLocation (Variables|Default|GetRootComponent_Player) (+ (Math|Vector|MakeVector (* AxisValue (Variables|Default|GetMoveSpeed)) 0.0 0.0) (Transformation|GetWorldLocation (Variables|Default|GetRootComponent_Player))) false false))

(event Input|AxisEvents|InputAxisMoveY
  (params (AxisValue :type Float%20%28single-precision%29))
  ;[1 1 1] Movement for sprite
  (Transformation|SetWorldLocation (Variables|Default|GetRootComponent_Player) (+ (Math|Vector|MakeVector 0.0 (* AxisValue (Variables|Default|GetMoveSpeed)) 0.0) (Transformation|GetWorldLocation (Variables|Default|GetRootComponent_Player))) false false))

(fn ConstructionScript)