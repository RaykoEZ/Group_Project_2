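; BP_Player is the player Blueprint, moving its sprite along world X and Y from input.
; The MoveX and MoveY axis events each scale the input by MoveSpeed and add it to the root component's world location.
; Movement sets the location directly without sweep or delta-time scaling, so it ignores blocking collision and depends on frame rate.
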(event Input|AxisEvents|InputAxisMoveX
  (params (AxisValue :type Float%20%28single-precision%29))
  ;[1 1 1] Movement for sprite
  (Transformation|SetWorldLocation (Variables|Default|GetRootComponent_Player) (+ (Math|Vector|MakeVector (* AxisValue (Variables|Components|GetMoveSpeed)) 0.0 0.0) (Transformation|GetWorldLocation (Variables|Default|GetRootComponent_Player))) false false))

(event Input|AxisEvents|InputAxisMoveY
  (params (AxisValue :type Float%20%28single-precision%29))
  ;[1 1 1] Movement for sprite
  (Transformation|SetWorldLocation (Variables|Default|GetRootComponent_Player) (+ (Math|Vector|MakeVector 0.0 (* AxisValue (Variables|Components|GetMoveSpeed)) 0.0) (Transformation|GetWorldLocation (Variables|Default|GetRootComponent_Player))) false false))

(fn ConstructionScript)